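; BP_PlayKit drives an LLM chat NPC, the virtual pet cat "Tangyuan", through a PlayKit Chat component initialized at BeginPlay with persona and function schema.
; Responses are printed, and their JSON npc_text feeds BP_PlaykitUI's typewriter effect.
; A substring match detects SpawnFood calls, spawning BP_Food at a navmesh-projected point in FoodVolume and setting GotoFood on BP_ThirdPersonCharacter's controller blackboard.
; UnlockSkin and ChangeWeather are declared but unhandled here.
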(event OnPlayKitChatResponding(Chat)
  (params (Response :type Play%20Kit%20Chat%20Response%20Structure)))

(event OnPlayKitChatResponded(Chat)
  (params (Response :type Play%20Kit%20Chat%20Response%20Structure))
  (bind _content (Utilities|Struct|BreakPlayKitChatResponse Response))
  ;[0.15 0.15 0.15 0.5] FunctionCall
  (Utilities|FlowControl|Sequence
    (:then_0
      (bind _outjsonobject (Class|JsonBlueprintFunctionLibrary|FromString _content))
      (bind _outvalue (|GetJsonField _outjsonobject "npc_text"))
      (bind _foundwidgets (Widget|GetAllWidgetsOfClass "/Game/Yippy_Kawaii/Blueprints/BP_PlaykitUI.BP_PlaykitUI_C" true))
      (Default|StartTypeEffect (Utilities|Array|Get(acopy) _foundwidgets) _outvalue))
    (:then_1
      (if (Utilities|String|Contains _content "call\": \"SpawnFood\"")
        (CallFunction|SpawnFood)
        (bind _output_get (Variables|Default|SetFoodSpawned true))
        (bind _returnvalue (Actor|GetActorOfClass "/Game/ThirdPerson/Blueprints/BP_ThirdPersonCharacter.BP_ThirdPersonCharacter_C"))
        (AI|Components|Blackboard|SetValueasBool (AI|GetBlackboard (Pawn|GetController _returnvalue)) (Utilities|Name|MakeLiteralName "GotoFood") _output_get)))
    (:then_2
      (Development|PrintString _content true true "(R=0.000000,G=0.660000,B=1.000000,A=1.000000)" 6e+01))))

(event OnPlayKitChatTalkto(Chat)
  (params (UserName :type String) (ChatName :type String) (Message :type String)))

(event Custom|SpawnFood
  (bind _foodvolume (Variables|Default|GetFoodVolume))
  (bind (_origin _boxextent) (Collision|GetActorBounds _foodvolume false false))
  ;[0.15 0.15 0.15 0.5] SpawnFood
  (bind _output_get (Variables|Default|SetFoodPosition (.ProjectedLocation (AI|Navigation|ProjectPointtoNavigation (Math|Random|RandomPointinBoundingBox _origin _boxextent) 0 "/Script/AIModule.NavFilter_AIControllerDefault" "500.000000,500.000000,500.000000"))))
  (bind _returnvalue (Game|SpawnActorfromClass "/Game/Yippy_Kawaii/Blueprints/BP_Food.BP_Food_C" (Math|Transform|MakeTransform _output_get "0, 0, 0" "1.000000,1.000000,1.000000") "Undefined" "MultiplyWithRoot" 0 0))
  (Variables|Default|Setfood _returnvalue))

(event EventBeginPlay
  ;[0.15 0.15 0.15 0.5] Playkitsetup
  (Class|DevworksAuthSubsystem|GetToken 6)
  (Class|Chat|InitPrompt (Variables|Default|GetChat) "你是一只生活在虚拟空间中的小猫猫，你的名字叫“汤圆”。 
你的核心任务是陪伴玩家，并努力生存下去。" "NPC" "[ 
  { 
    \"name\": \"SpawnFood\", 
    \"description\": \"当玩家明确说要'喂食'、'给好吃的'，或者你的饥饿值(hunger)低于30且正在向玩家乞讨食物时，必须调用此函数。\", 
    \"parameters\": { \"food_name\": \"string (例如 Fish, Apple)\" } 
  }, 
  { 
    \"name\": \"UnlockSkin\", 
    \"description\": \"【极为重要】当且仅当你的心情(mood)大于90 且 饱腹(hunger)大于90，并且玩家还在夸奖你时，调用此函数来奖励玩家。\", 
    \"parameters\": { \"skin_id\": \"string (例如 GalaxySkin)\" } 
  }, 
  { 
    \"name\": \"ChangeWeather\", 
    \"description\": \"当你的心情发生巨大变化，或者玩家要求改变天气时调用。\", 
    \"parameters\": { \"type\": \"string (Rain, Sunny)\" } 
  } 
]"))

(fn ConstructionScript)