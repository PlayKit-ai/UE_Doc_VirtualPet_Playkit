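; BP_SpawnFood is a spawner actor that places a BP_Food actor at a random navigable spot within a volume.
; BeginPlay starts a timeline whose updates pass a threshold check into a DoOnce with no reset, so food spawns only once.
; It picks a random point in the Volume's bounds, projects it onto the navmesh, spawns the food there and stores the reference.
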(event EventBeginPlay
  (bind _volume (Variables|Default|GetVolume))
  (bind (_origin _boxextent) (Collision|GetActorBounds _volume false false))
  (bind _newtrack_0 (Timeline|Timeline Play)
    (:Update
      (if (< _newtrack_0 15.0)
        (Utilities|FlowControl|DoOnce false
          (:Completed
            (bind _output_get (Variables|Default|SetFoodPosition (.ProjectedLocation (AI|Navigation|ProjectPointtoNavigation (Math|Random|RandomPointinBoundingBox _origin _boxextent) 0 "/Script/AIModule.NavFilter_AIControllerDefault" "500.000000,500.000000,500.000000"))))
            (bind _returnvalue (Game|SpawnActorfromClass "/Game/Yippy_Kawaii/Blueprints/BP_Food.BP_Food_C" (Math|Transform|MakeTransform _output_get "0, 0, 0" "1.000000,1.000000,1.000000") "Undefined" "MultiplyWithRoot" 0 0))
            (Variables|Default|SetFood _returnvalue)))))))

(event Collision|EventActorBeginOverlap
  (params (OtherActor :type Actor%20Object%20Reference)))

(fn ConstructionScript)